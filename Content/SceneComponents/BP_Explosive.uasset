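; BP_Explosive is an actor that explodes when it takes any damage, then destroys itself.
; It applies full radial damage within ExplosionRadius, ignoring itself and the pawn controlled by the damage instigator, who is credited for the blast.
; The construction script sizes Sphere to that radius, but the overlap only feeds a debug print of the BP_Character count.
; An ApplyDamage node is left unconnected.
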(event `self.ReceiveAnyDamage`
  (params (Damage :type "Float (single-precision)") (DamageType :type "DamageType Object Reference") (InstigatedBy :type "Controller Object Reference") (DamageCauser :type "Actor Object Reference"))
  (bind _returnvalue_location (`KismetMathLibrary.BreakTransform` (`self.GetTransform`)))
  (`KismetSystemLibrary.PrintString` (`KismetStringLibrary.Conv_IntToString` (`KismetArrayLibrary.Array_Length` (`PrimitiveComponent.GetOverlappingActors` (`self.Sphere`) "/Game/Character/BP_Character.BP_Character_C"))))
  (`GameplayStatics.ApplyRadialDamage` (`self.Damage`) _returnvalue_location (`self.ExplosionRadius`) null (`|MakeArray` self (`Controller.K2_GetPawn` InstigatedBy) :!type "Actor Object Reference") DamageCauser InstigatedBy true)
  (`self.K2_DestroyActor`))

(fn `UserConstructionScript`
  (`SphereComponent.SetSphereRadius` (`self.Sphere`) (`self.ExplosionRadius`) true))