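; BP_Spectator_Free is a free-moving spectator that flies through the level along the controller's facing.
; BeginPlay runs the parent logic, then collapses the SpringArm to zero length.
; MoveForward and MoveRight axis inputs offset the actor transform directly along the controller's forward and right vectors, using a fixed step with no delta-time scaling or sweep.
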(event `InputAxis|MoveForward`
  (params (AxisValue :type "Float (single-precision)"))
  (bind (_returnvalue_location _returnvalue_rotation _returnvalue_scale) (`KismetMathLibrary.BreakTransform` (`self.GetTransform`)))
  (`self.K2_SetActorTransform` (`KismetMathLibrary.MakeTransform` (+ (* (`self.GetActorForwardVector` (`self.GetController`)) (* AxisValue 20.0)) _returnvalue_location) _returnvalue_rotation _returnvalue_scale)))

(event `self.ReceiveBeginPlay`
  (`parent.ReceiveBeginPlay`)
  (set `SpringArmComponent.TargetArmLength` 0.0 (`self.SpringArm`)))

(event `InputAxis|MoveRight`
  (params (AxisValue :type "Float (single-precision)"))
  (bind (_returnvalue_location _returnvalue_rotation _returnvalue_scale) (`KismetMathLibrary.BreakTransform` (`self.GetTransform`)))
  (`self.K2_SetActorTransform` (`KismetMathLibrary.MakeTransform` (+ (* (`self.GetActorRightVector` (`self.GetController`)) (* AxisValue 20.0)) _returnvalue_location) _returnvalue_rotation _returnvalue_scale)))

(fn `UserConstructionScript`
  (`parent.UserConstructionScript`))