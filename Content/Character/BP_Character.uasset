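; Networked first-person shooter character with move and look input, a replicated weapon and ragdoll death.
; On possession the server spawns BP_Weapon, and its OnRep attaches it to the arms mesh for the local player or the body mesh otherwise.
; Fire input goes to a server event that uses the weapon's trace to apply point damage and draw debug shapes.
; The Dead OnRep disables movement, ragdolls the body, destroys the weapon and schedules actor destruction.
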(event `InputAxis|LookUp`
  (params (AxisValue :type "Float (single-precision)"))
  (`self.AddControllerPitchInput` AxisValue))

(event `InputAxis|MoveForward`
  (params (AxisValue :type "Float (single-precision)"))
  (`self.AddMovementInput` (`self.GetActorForwardVector`) AxisValue))

(event `InputAxis|Turn`
  (params (AxisValue :type "Float (single-precision)"))
  (`self.AddControllerYawInput` AxisValue))

(event `InputAxis|MoveRight`
  (params (AxisValue :type "Float (single-precision)"))
  (`self.AddMovementInput` (`self.GetActorRightVector`) AxisValue))

(event `self.ReceivePossessed`
  (params (NewController :type "Controller Object Reference"))
  (`/Engine/EditorBlueprintResources/ActorMacros.Switch Has Authority`
    (:`Authority`
      (bind _weapon (`self.CreateWeapon`))
      (set `self.Weapon` _weapon))))

(event `InputAction|Fire`
  (params (Key :type "Key Structure"))
  (:`Pressed`
    (`self.Server_Fire`)))

(event `DEBUG_DrawServerTrace`
  (params (LineStart :type "Vector Structure") (LineEnd :type "Vector Structure") (Center :type "Vector Structure"))
  (`KismetSystemLibrary.DrawDebugLine` LineStart LineEnd (struct :`R` 1.0 :`G` 0.827258 :`A` 1.0) 5.0 0.5)
  (`KismetSystemLibrary.DrawDebugSphere` Center 5.0 12 (struct :`R` 1.0 :`B` 0.014042 :`A` 1.0) 5.0 0.5))

(event `Server_Fire`
  (bind _weapon (`self.Weapon`))
  (bind _hit (`/Game/Character/BP_Weapon.Get Trace` (`self.Weapon`)))
  (bind (_bblockinghit _binitialoverlap _time _distance _location _impactpoint _normal _impactnormal _physmat _hitactor _hitcomponent _hitbonename _hititem _faceindex _tracestart _traceend) (`GameplayStatics.BreakHitResult` _hit))
  (`self.DEBUG_DrawServerTrace` _tracestart _traceend _location)
  (`GameplayStatics.ApplyPointDamage` _hitactor (`/Game/Character/BP_Weapon.Damage` _weapon) (`KismetMathLibrary.GetDirectionUnitVector` _traceend _tracestart) _hit (`self.GetController`) _weapon))

(fn `CreateWeapon`
  (returns (Weapon :type "/Game/Character/BP_Weapon Object Reference"))
  (bind _returnvalue (`|SpawnActorFromClass` "/Game/Character/BP_Weapon.BP_Weapon_C" (`KismetMathLibrary.MakeTransform` (0.0 0.0 0.0)) "AlwaysSpawn" "OverrideRootScale" (`self.GetController`) self))
  (`self.K2_AttachToActor` _returnvalue self "None" "SnapToTarget" "SnapToTarget" "SnapToTarget" true)
  (return _returnvalue))

(fn `Destroy`
  (`self.K2_DestroyActor`))

(fn `GetVisibleMesh`
  (returns (`Skeletal Mesh` :type "SkeletalMeshComponent Object Reference"))
  (return (select `bool` (`self.IsLocallyControlled`) :`false` (`self.BodyMesh`) :`true` (`self.ArmsMesh`))))

(fn `OnRep_Dead`
  (if (`self.Dead`)
    (`self.CharacterDead`)
    (`CharacterMovementComponent.DisableMovement` (`self.CharacterMovement`))
    (`PrimitiveComponent.SetCollisionEnabled` (`self.CapsuleComponent`) "NoCollision")
    (`PrimitiveComponent.SetSimulatePhysics` (`self.BodyMesh`) true)
    (`PrimitiveComponent.SetCollisionEnabled` (`self.BodyMesh`) "QueryAndPhysics")
    (bind _weapon (`self.Weapon`)
      (:`then`
        (`self.K2_DestroyActor` _weapon))
      (:`else`
        _))
    (`KismetSystemLibrary.K2_SetTimer` null "Destroy" (`self.DestroyTime`))))

(fn `OnRep_Weapon`
  (`self.Weapon`
    (:`then`
      (if true
        (`self.K2_AttachToComponent` (`self.Weapon`) (`self.GetVisibleMesh`) "hand_rSocket" "KeepRelative" "KeepRelative" "KeepRelative" true)))
    (:`else`)))

(fn `UserConstructionScript`)