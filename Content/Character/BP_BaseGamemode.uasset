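; Base game mode that handles character death, spectating and player spawning.
; On death it fires CallCharDead, then, for player-controlled characters, starts the controller's respawn timer and possesses a spectator.
; The spectator follows the killer when the instigator is valid, otherwise it is free-roaming at the death location.
; Spawning picks a random free BP_PlayerStart, falling back to any start when none are free.
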(fn `CharacterDead`
  (params (DeadCharacter :type "/Game/Character/BP_Character Object Reference") (DeathInstigator :type "/Game/Character/BP_PlayerController Object Reference") (DeathCauseBy :type "Actor Object Reference"))
  (`self.CharDead` DeadCharacter DeathInstigator DeathCauseBy)
  (bind _asbp_player_controller (cast `/Game/Character/BP_PlayerController` (`Pawn.GetController` DeadCharacter)))
  (`|ExecutionSequence`
    (:`then_0`
      (`/Game/Character/BP_PlayerController.StartRespawnTimer` _asbp_player_controller (`self.RespawnTime`)))
    (:`then_1`
      (`self.OnDeadSpawnSpectator` _asbp_player_controller DeathInstigator))))

(fn `GetAvailableSpawnPoints`
  (returns (AvailableSpawns :type "Array of /Game/Character/BP_PlayerStart Object Reference"))
  (locals (Result :type "Array of /Game/Character/BP_PlayerStart Object Reference"))
  (bind _outactors (`GameplayStatics.GetAllActorsOfClass` "/Game/Character/BP_PlayerStart.BP_PlayerStart_C"))
  (for _array_element _outactors
    (if (`/Game/Character/BP_PlayerStart.IsFree` _array_element)
      (`KismetArrayLibrary.Array_Add` (`local.Result`) _array_element)))
  (return (`local.Result`)))

(fn `OnDeadSpawnSpectator`
  (params (Player :type "/Game/Character/BP_PlayerController Object Reference") (DeathInstigator :type "/Game/Character/BP_PlayerController Object Reference"))
  (returns (Spectator :type "/Game/Spectator/BP_Spectator Object Reference"))
  (bind _returnvalue (`KismetSystemLibrary.IsValid` DeathInstigator))
  (bind _returnvalue_2 (`Controller.K2_GetPawn` DeathInstigator))
  (bind _spectator (`self.SpawnSpectator` Player (select `bool` _returnvalue :`false` "/Game/Spectator/BP_Spectator_Free.BP_Spectator_Free_C" :`true` "/Game/Spectator/BP_Spectator_CharFollow.BP_Spectator_CharFollow_C" :!type "/Game/Spectator/BP_Spectator Class Reference") (`self.GetTransform` (select `bool` _returnvalue :`false` (`Controller.K2_GetPawn` Player) :`true` _returnvalue_2))))
  (bind _asbp_spectator_char_follow (cast `/Game/Spectator/BP_Spectator_CharFollow` _spectator)
    (:`then`
      (set `/Game/Spectator/BP_Spectator_CharFollow.FollowCharacter` (cast `/Game/Character/BP_Character` _returnvalue_2 :!pure true) _asbp_spectator_char_follow))
    (:`CastFailed`
      _))
  (return _spectator))

(fn `SpawnPlayer`
  (params (Player :type "/Game/Character/BP_PlayerController Object Reference"))
  (locals (L_PlayerStart :type "/Game/Character/BP_PlayerStart Object Reference"))
  (bind _availablespawns (`self.GetAvailableSpawnPoints`))
  (bind _returnvalue (> (`KismetArrayLibrary.Array_Length` _availablespawns) 0))
  (if (not _returnvalue)
    (bind _outactors (`GameplayStatics.GetAllActorsOfClass` "/Game/Character/BP_PlayerStart.BP_PlayerStart_C")))
  (`/Game/Character/BP_PlayerStart.SpawnCharacter` (select `bool` _returnvalue :`false` (`|GetArrayItem` _outactors (`KismetMathLibrary.RandomInteger` (`KismetArrayLibrary.Array_LastIndex` _outactors))) :`true` (`|GetArrayItem` _availablespawns (`KismetMathLibrary.RandomInteger` (`KismetArrayLibrary.Array_LastIndex` _availablespawns)))) Player))

(fn `SpawnSpectator`
  (params (Player :type "/Game/Character/BP_PlayerController Object Reference") (`Spectator Class` :type "/Game/Spectator/BP_Spectator Class Reference") (SpawnTransform :type "Transform Structure"))
  (returns (Spectator :type "/Game/Spectator/BP_Spectator Object Reference"))
  (bind _returnvalue (`|SpawnActorFromClass` `Spectator Class` SpawnTransform "Undefined" "OverrideRootScale" Player null))
  (`Controller.Possess` Player _returnvalue)
  (return _returnvalue))

(fn `UserConstructionScript`)