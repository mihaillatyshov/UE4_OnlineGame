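; BP_Weapon is a weapon actor that provides an aiming line trace for the character using it.
; It casts its Instigator to BP_Character and caches it, in both the Construction Script and BeginPlay.
; GetTrace runs a long object trace from that character's camera along the owner's forward vector, not the camera's.
; It targets world static, world dynamic and pawn objects, ignores itself and the Instigator, and returns the hit.
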(event `self.ReceiveBeginPlay`
  (bind _asbp_character (cast `/Game/Character/BP_Character` (`self.GetInstigator`)))
  (set `self.Character` _asbp_character))

(fn `Get Trace`
  (returns (Hit :type "HitResult Structure"))
  (bind _returnvalue (`SceneComponent.K2_GetComponentLocation` (`/Game/Character/BP_Character.Camera` (`self.Character`))))
  (bind _outhit (`KismetSystemLibrary.LineTraceSingleForObjects` _returnvalue (+ _returnvalue (* (`self.GetActorForwardVector` (`self.GetOwner`)) 100000.0)) (`|MakeArray` "ObjectTypeQuery1" "ObjectTypeQuery2" "ObjectTypeQuery3" :!type "EObjectTypeQuery Enum") false (`|MakeArray` self (`self.GetInstigator`) :!type "Actor Object Reference")))
  (return _outhit))

(fn `UserConstructionScript`
  (bind _asbp_character (cast `/Game/Character/BP_Character` (`self.GetInstigator`)))
  (set `self.Character` _asbp_character))