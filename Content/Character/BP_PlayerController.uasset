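; Player controller that handles switching between playing and spectating, plus local UI and input mode.
; Server_Respawn flags the player state as a player and asks BP_BaseGamemode to spawn it, while Server_Spectator requests a free spectator at the controller's transform.
; StartRespawnTimer schedules a delayed respawn.
; Local BeginPlay adds the leaderboard and shows the cursor; WidgetSetup enters game-only input, and an input action toggles between game and UI modes.
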(event `InputAction|MouseCursorVis`
  (params (Key :type "Key Structure"))
  (:`Released`
    (bind _output_get (set `self.IsInGame` (not (`self.IsInGame`))))
    (if _output_get
      (`WidgetBlueprintLibrary.SetInputMode_GameOnly` self)
      (set `self.bShowMouseCursor` false)
      (else
        (`WidgetBlueprintLibrary.SetInputMode_UIOnlyEx` null null)
        (set `self.bShowMouseCursor` true)))))

(event `Key|Enter`
  (params (Key :type "Key Structure")))

(event `Server_Respawn`
  (bind _asbp_player_state (cast `/Game/Character/BP_PlayerState` (`self.PlayerState`)))
  (set `/Game/Character/BP_PlayerState.IsPlayer` true _asbp_player_state)
  (`self.Respawn`))

(event `Server_Spectator`
  (`self.Respawn_Spectator`))

(event `self.ReceiveBeginPlay`
  (if (`self.IsLocalPlayerController`)
    (set `self.bShowMouseCursor` true)
    (bind _returnvalue (`|CreateWidget` "/Game/Character/BP_Leaderboard.BP_Leaderboard_C" self))
    (bind _output_get (set `self.Leaderboard` _returnvalue))
    (`UserWidget.AddToViewport` _output_get 0)))

(fn `Respawn`
  (bind _asbp_base_gamemode (cast `/Game/Character/BP_BaseGamemode` (`GameplayStatics.GetGameMode`)))
  (`/Game/Character/BP_BaseGamemode.SpawnPlayer` _asbp_base_gamemode self))

(fn `Respawn_Spectator`
  (bind _asbp_base_gamemode (cast `/Game/Character/BP_BaseGamemode` (`GameplayStatics.GetGameMode`)))
  (`/Game/Character/BP_BaseGamemode.SpawnSpectator` _asbp_base_gamemode self "/Game/Spectator/BP_Spectator_Free.BP_Spectator_Free_C" (`self.GetTransform`)))

(fn `StartRespawnTimer`
  (params (Time :type "Float (double-precision)"))
  (bind _returnvalue (`KismetSystemLibrary.K2_SetTimer` null "Respawn" Time))
  (set `self.RespawnTimer` _returnvalue))

(fn `UserConstructionScript`)

(fn `WidgetSetup`
  (set `self.bShowMouseCursor` false)
  (`WidgetBlueprintLibrary.SetInputMode_GameOnly` self)
  (set `self.IsInGame` true))